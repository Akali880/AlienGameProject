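; Shooting target enemy that turns to face the first-person character when its PlayerDetection component sees it, then attacks.
; Each attack spawns a projectile at SpawnProjectileLocation and applies damage directly to the player without waiting for impact, then a Delay-based CanAttack flag enforces a cooldown.
; HitEnemy subtracts damage from Health, printing the remainder or destroying the actor; its death check subtracts Damage again from the updated Health.
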(event `self.PlayerDetection.OnSeePawn`
  (params (Pawn :type "Pawn Object Reference"))
  ;[1 1 1] Target Shooting Logic
  (bind _asbp_first_person_character (cast `/Game/FirstPerson/Blueprints/BP_FirstPersonCharacter` Pawn))
  (`self.K2_SetActorRotation` (`KismetMathLibrary.FindRelativeLookAtRotation` (`KismetMathLibrary.Conv_VectorToTransform` (`self.K2_GetActorLocation`)) (`self.K2_GetActorLocation` _asbp_first_person_character)))
  (if (`self.CanAttack?`)
    (`|SpawnActorFromClass` "/Game/FirstPerson/Blueprints/BP_FirstPersonProjectile.BP_FirstPersonProjectile_C" (`SceneComponent.K2_GetComponentToWorld` (`self.SpawnProjectileLocation`)) "Undefined" "MultiplyWithRoot" null null)
    (`GameplayStatics.ApplyDamage` _asbp_first_person_character 20.0)
    (set `self.CanAttack?` false)
    (`KismetSystemLibrary.Delay` 2.0)
    (set `self.CanAttack?` true)))

(event `/Game/Targets/EnemyDamage_Interface.HitEnemy`
  (params (Damage :type "Float (double-precision)"))
  (bind _returnvalue (- (`self.Health`) Damage))
  ;[1 1 1] Damage + Death Logic
  (bind _output_get (set `self.Health` _returnvalue))
  (if (<= _returnvalue 0.0)
    (`KismetSystemLibrary.PrintString` "EnemyKilled")
    (`self.K2_DestroyActor`)
    (else
      (`KismetSystemLibrary.PrintString` (`KismetStringLibrary.Conv_DoubleToString` _output_get)))))

(fn `UserConstructionScript`)