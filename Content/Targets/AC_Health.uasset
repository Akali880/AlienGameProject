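; Health component (AC_Health) that tracks current HP, with restore, removal, optional regeneration and death notification.
; A looping timer started at BeginPlay drives regeneration, pausing at max HP and unpausing after non-lethal removal.
; RemoveHP subtracts current HP from the incoming amount, reversed from usual damage math, so amounts at or below current HP trigger death.
; Death is broadcast through an event dispatcher call.
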(event `self.ReceiveBeginPlay`
  ;[1 1 1] Decides If Player Needs to Regenerate Health Points or Not
  (if (`self.ShouldRegen?`)
    (bind _returnvalue (`KismetSystemLibrary.K2_SetTimer` null "RegenHP" (`self.RegenRate`) true))
    (set `self.RegenTimer` _returnvalue)))

(event `Death`
  ;[1 1 1] Death Logic
  (`self.DeathDispatcher`))

(fn `RegenHP`
  (bind _returnvalue (+ (`self.CurrentHP`) (`self.RegenAmount`)))
  ;[1 1 1] Health Point Regeneration Logic
  (if (`self.ShouldRegen?`)
    (if (>= _returnvalue (`self.MaxHP`))
      (set `self.CurrentHP` (`self.MaxHP`))
      (`KismetSystemLibrary.K2_PauseTimerHandle` (`self.RegenTimer`))
      (else
        (set `self.CurrentHP` _returnvalue)))))

(fn `RemoveHP`
  (params (AmountToRemove :type "Float (double-precision)"))
  (bind _returnvalue (- AmountToRemove (`self.CurrentHP`)))
  ;[1 1 1] Heatlh Point Decrease Logic
  (if (<= _returnvalue 0.0)
    (`self.Death`)
    (else
      (set `self.CurrentHP` _returnvalue)
      (if (< (`self.CurrentHP`) (`self.MaxHP`))
        (`KismetSystemLibrary.K2_UnPauseTimerHandle` (`self.RegenTimer`))))))

(fn `RestoreHP`
  (params (AmountToRestore :type "Float (double-precision)"))
  (bind _returnvalue (+ (`self.CurrentHP`) AmountToRestore))
  ;[1 1 1] Health Point Increase Logic
  (if (>= _returnvalue (`self.MaxHP`))
    (set `self.CurrentHP` (`self.MaxHP`))
    (else
      (set `self.CurrentHP` _returnvalue))))